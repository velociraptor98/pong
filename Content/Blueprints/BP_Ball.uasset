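; BP_Ball is a Pong-style ball that bounces off paddles and boundaries by rewriting its sphere's physics velocity.
; Actor overlap events route to HitPaddle or HitBoundary by casting the other actor.
; A boundary hit inverts vertical (Z) velocity and adds random jitter.
; A paddle hit reverses X and replaces Z with a randomly scaled-down share of the paddle collider's vertical velocity, plus jitter.
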(event Collision|EventActorBeginOverlap
  (params (OtherActor :type Actor%20Object%20Reference))
  ;[1 1 1] collision
  (bind _aspaddle (Utilities|Casting|CastToPaddle OtherActor)
    (:then
      (Class|Ball|HitPaddle _aspaddle))
    (:CastFailed
      (Utilities|Casting|CastToBoundary OtherActor)
      (Class|Ball|HitBoundary))))

(event EventHitPaddle
  (params (Paddle :type Paddle%20Object%20Reference))
  ;[1 1 1] on hitting paddle
  (bind _returnvalue (Physics|GetPhysicsLinearVelocity (Variables|/Script/Pong.Paddle|GetCollider Paddle) "None"))
  (bind _returnvalue_2 (Physics|GetPhysicsLinearVelocity (Variables|Default|GetSphere) "None"))
  (Physics|SetPhysicsLinearVelocity (Variables|Default|GetSphere) (Math|Vector|MakeVector (* (.x _returnvalue_2) -1.0) (.y _returnvalue_2) (+ (/ (.z _returnvalue) (Math|Random|RandomFloatinRange 2.0 3.0)) (Math|Random|RandomFloatinRange -2e+02 2e+02))) false "None"))

(event EventHitBoundary
  ;[1 1 1] on hitting boundary
  (bind _returnvalue (Physics|GetPhysicsLinearVelocity (Variables|Default|GetSphere) "None"))
  (Physics|SetPhysicsLinearVelocity (Variables|Default|GetSphere) (Math|Vector|MakeVector (.x _returnvalue) (.y _returnvalue) (+ (* (.z _returnvalue) -1.0) (Math|Random|RandomFloatinRange -2e+02 2e+02))) false "None"))

(fn ConstructionScript)