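; BP_PaddleAi is the computer-controlled paddle in a Pong game.
; Each tick it reads the ball reference from PongGameMode and checks the ball's X velocity.
; When the ball moves toward positive X, it follows the ball's Z at MoveSpeed with a swept move on a fixed X and Y.
; Otherwise it returns to center height at double speed without sweeping, using constant-speed interpolation in both cases.
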(event EventTick
  (params (DeltaSeconds :type Float%20%28single-precision%29))
  ;[1 1 1] ai paddle
  (bind _aspong_game_mode (Utilities|Casting|CastToPongGameMode (Game|GetGameMode)))
  (bind _output_get (Variables|Default|SetBallRef (Variables|/Script/Pong.PongGameMode|GetBallRef _aspong_game_mode)))
  (Utilities|IsValid _output_get
    (:Is%20Valid
      (if (> (.x (Transformation|GetVelocity _output_get)) 0.0)
        (Transformation|SetActorLocation (Math|Interpolation|VInterptoConstant (Transformation|GetActorLocation) (Math|Vector|MakeVector 8.5e+02 1e+01 (.z (Transformation|GetActorLocation (Variables|Default|GetBallRef)))) (Utilities|Time|GetWorldDeltaSeconds) (Variables|Default|GetMoveSpeed)) true false)
        (else
          (Transformation|SetActorLocation (Math|Interpolation|VInterptoConstant (Transformation|GetActorLocation) (Math|Vector|MakeVector 8.5e+02 1e+01 0.0) (Utilities|Time|GetWorldDeltaSeconds) (* (Variables|Default|GetMoveSpeed) 2.0)) false false))))))

(fn ConstructionScript)