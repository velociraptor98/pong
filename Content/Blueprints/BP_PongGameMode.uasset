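; BP_PongGameMode runs a Pong match, tracking AI and player scores and managing ball spawns.
; On BeginPlay it creates the HUD widget and serves the first ball in a random horizontal direction.
; Score events increment a counter, update the HUD, set the next serve direction by scorer, and respawn the ball.
; Each spawn uses short delays before launching the ball by setting its sphere's physics linear velocity along X.
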(event EventBeginPlay
  ;[1 1 1] create widget and spawn ball
  (bind _returnvalue (UserInterface|CreateWidget "/Game/Blueprints/BP_GameHUD.BP_GameHUD_C"))
  (bind _output_get (Variables|Default|SetGameHUDref _returnvalue))
  (UserInterface|Viewport|AddtoViewport _output_get 0)
  (Variables|Default|SetDirection (Math|Float|Sign(Float) (Math|Random|RandomFloatinRange -1.0 1.0)))
  (Class|PongGameMode|SpawnBall))

(event EventIncreaseAiScore
  ;[1 1 1] update score when ball is destroyed
  (bind _result (Math|Integer|IncrementInt (Variables|Default|GetAiScore))
    (:%20%20
      (Class|GameHUD|UpdateAiScore (Variables|Default|GetGameHUDref) _result)
      (Variables|Default|SetDirection -1.0)
      (Class|PongGameMode|SpawnBall))))

(event EventSpawnBall
  ;[1 1 1] spawn ball
  (Utilities|FlowControl|Delay 1.0)
  (bind _returnvalue (Game|SpawnActorfromClass "/Game/Blueprints/BP_Ball.BP_Ball_C" (Math|Transform|MakeTransform "0,10.000000, 0" "0, 0, 0" "1,1,1") "AlwaysSpawn" 0 0))
  (bind _output_get (Variables|Default|SetBallRef _returnvalue))
  (Utilities|FlowControl|Delay 0.5)
  (Physics|SetPhysicsLinearVelocity (Variables|/Script/Pong.Ball|GetSphere _output_get) (Math|Vector|MakeVector (* (Variables|Default|GetDirection) (Variables|Default|GetBallSpeed)) 0.0 0.0) false "None"))

(event EventIncreasePlayerScore
  ;[1 1 1] update score when ball is destroyed
  (bind _result (Math|Integer|IncrementInt (Variables|Default|GetPlayerScore))
    (:%20%20
      (Class|GameHUD|UpdatePlayerScore (Variables|Default|GetGameHUDref) _result)
      (Variables|Default|SetDirection 1.0)
      (Class|PongGameMode|SpawnBall))))

(fn ConstructionScript)