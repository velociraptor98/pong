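; BP_Boundary is a boundary actor for a Pong game that can act as a scoring goal when flagged with IsGoal.
; It caches the PongGameMode on BeginPlay.
; When a Ball overlaps a goal, it destroys the ball and calls the game mode to increase the AI score for the left goal, otherwise the player's score.
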(event EventBeginPlay
  ;[1 1 1] ref to game mode
  (bind _aspong_game_mode (Utilities|Casting|CastToPongGameMode (Game|GetGameMode)))
  (Variables|Default|SetGameModeref _aspong_game_mode))

(event Collision|EventActorBeginOverlap
  (params (OtherActor :type Actor%20Object%20Reference))
  (bind _gamemoderef (Variables|Default|GetGameModeref))
  ;[1 1 1] Comment
  (if (Variables|Default|GetisGoal)
    (bind _asball (Utilities|Casting|CastToBall OtherActor))
    (Actor|DestroyActor _asball)
    (if (Variables|Default|GetisLeftGoal)
      (Class|PongGameMode|IncreaseAiScore _gamemoderef)
      (else
        (Class|PongGameMode|IncreasePlayerScore _gamemoderef)))))

(fn ConstructionScript)